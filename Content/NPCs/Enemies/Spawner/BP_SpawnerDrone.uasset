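; BP_SpawnerDrone is a spawner's drone enemy that circles the spawner's start location and reports its destruction to that spawner.
; After a zero-second delay at BeginPlay, the Orbit timeline sweeps yaw a full turn from the initial heading, setting position at a fixed radius and matching rotation.
; On Destroyed, it calls UpdateMiniBoss on the owning BP_SpawnerEnemy.
; The construction script removes the Mesh component; a Cube hover timeline exists but never runs.
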(event `self.ReceiveBeginPlay`
  (bind (_returnvalue_roll _returnvalue_pitch _returnvalue_yaw) (`KismetMathLibrary.BreakRotator` (`self.K2_GetActorRotation`)))
  (bind _initialyaw (`self.InitialYaw`))
  (`parent.ReceiveBeginPlay`)
  (`KismetSystemLibrary.Delay` 0.0)
  (set `self.InitialYaw` _returnvalue_yaw)
  (bind (_direction _alpha) (`Timeline|Orbit` :!via `PlayFromStart`)
    (:`Update`
      (bind _returnvalue (`KismetMathLibrary.Lerp` _initialyaw (+ _initialyaw 360.0) _alpha))
      (`self.K2_SetActorLocationAndRotation` (+ (`self.SpawnerStartLocation`) (`KismetMathLibrary.LessLess_VectorRotator` (1000.0 0.0 0.0) (`KismetMathLibrary.MakeRotator` 0.0 0.0 _returnvalue))) (`KismetMathLibrary.MakeRotator` 0.0 0.0 _returnvalue)))))

(event `self.ReceiveDestroyed`
  (bind _asbp_spawner_enemy (cast `/Game/NPCs/Enemies/Spawner/BP_SpawnerEnemy` (`self.OwnerSpawner`)))
  (`/Game/NPCs/Enemies/Spawner/BP_SpawnerEnemy.UpdateMiniBoss` _asbp_spawner_enemy self))

(fn `UserConstructionScript`
  (`parent.UserConstructionScript`)
  (`ActorComponent.K2_DestroyComponent` (`self.Mesh`)))