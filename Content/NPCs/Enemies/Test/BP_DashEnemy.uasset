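; BP_DashEnemy is an enemy NPC in a Test folder that damages the player with a dash attack.
; When the DashCollision component overlaps the player during an attack dash, it sets itself as BP_Player's Attacker and calls Hit.
; The Dash event only runs a debug-drawn box trace from the actor's location; its result is unused and no movement happens here.
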(event `self.DashCollision.OnComponentBeginOverlap`
  (params (OverlappedComponent :type "PrimitiveComponent Object Reference") (OtherActor :type "Actor Object Reference") (OtherComp :type "PrimitiveComponent Object Reference") (OtherBodyIndex :type Integer) (bFromSweep :type Boolean) (SweepResult :type "HitResult Structure (by ref)"))
  (bind _returnvalue (`GameplayStatics.GetPlayerCharacter` 0))
  (if (`self.IsAttackDashing`)
    (if (== OtherActor _returnvalue)
      (bind _asbp_player (cast `/Game/Player/PlayerBlueprint/BP_Player` _returnvalue))
      (set `/Game/Gameplay/BP_CharacterParent.Attacker` self _asbp_player)
      (`self.Hit` _asbp_player))))

(event `Dash`
  (`KismetSystemLibrary.BoxTraceSingle` :`Start` (`self.K2_GetActorLocation`) :`HalfSize` (40.0 40.0 90.0) :`TraceChannel` "TraceTypeQuery1" :`DrawDebugType` "ForDuration"))

(fn `UserConstructionScript`
  (`parent.UserConstructionScript`))