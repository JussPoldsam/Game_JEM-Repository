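; BP_SpawnerEnemy is a test enemy with five rotating cannons that fire projectiles, sweep lasers and spawn enemies.
; BeginPlay rings the cannon meshes, then the RotatingCannons timeline spins them, firing normal or enemy-spawning physics projectiles on event tracks.
; After one shot, its laser track hands over to the Laser timeline, whose debug-drawn traces only print on player hits, then resumes rotation.
; On destruction it spawns five BP_TestEnemy01 in a ring; the Scale timeline is never triggered.
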(event `self.ReceiveBeginPlay`
  (`parent.ReceiveBeginPlay`)
  (bind _output_get (set `self.Meshes` (`|MakeArray` (`self.Mesh1`) (`self.Mesh2`) (`self.Mesh3`) (`self.Mesh4`) (`self.Mesh5`))))
  (for (_array_element _array_index) _output_get
    (`SceneComponent.K2_SetRelativeLocation` _array_element (`KismetMathLibrary.GreaterGreater_VectorRotator` (65.0 0.0 0.0) (`KismetMathLibrary.MakeRotator` 0.0 0.0 (/ (* _array_index 360.0) 5.0))) false false)
    (bind (_returnvalue_roll _returnvalue_pitch _returnvalue_yaw) (`KismetMathLibrary.BreakRotator` (`KismetMathLibrary.FindLookAtRotation` (`SceneComponent.K2_GetComponentLocation` _array_element) (`self.K2_GetActorLocation`))))
    (`SceneComponent.K2_SetWorldRotation` _array_element (`KismetMathLibrary.MakeRotator` 0.0 0.0 (+ _returnvalue_yaw 180.0)) false false)
    (bind (_direction _yaw) (`Timeline|RotatingCannons` :!label _label)
      (:`Update`
        (`SceneComponent.K2_SetRelativeRotation` (`self.Rotator`) (`KismetMathLibrary.MakeRotator` 0.0 0.0 _yaw) false false))
      (:`Attack`
        (set `self.Shots` (+ (`self.Shots`) 1))
        (for _array_element_2 (`self.Meshes`)
          (bind (_returnvalue_roll_2 _returnvalue_pitch_2 _returnvalue_yaw_2) (`KismetMathLibrary.BreakRotator` (`KismetMathLibrary.FindLookAtRotation` (`self.K2_GetActorLocation`) (`SceneComponent.K2_GetComponentLocation` _array_element_2))))
          (bind _returnvalue (`|SpawnActorFromClass` "/Game/Gameplay/Attacks/EnemyAttacks/BP_EnemySpawnerProjectile.BP_EnemySpawnerProjectile_C" (`KismetMathLibrary.MakeTransform` (+ (`SceneComponent.K2_GetComponentLocation` _array_element_2) (`KismetMathLibrary.GreaterGreater_VectorRotator` (10.0 0.0 0.0) (`KismetMathLibrary.MakeRotator` 0.0 0.0 _returnvalue_yaw_2)))) "Undefined" "OverrideRootScale" null null))
          (set `/Game/Gameplay/Attacks/BP_ProjectileParent.Shooter` self _returnvalue)
          (`PrimitiveComponent.AddImpulse` (`/Game/Gameplay/Attacks/BP_ProjectileParent.PhysicsCube` _returnvalue) (`KismetMathLibrary.GreaterGreater_VectorRotator` (1000.0 0.0 0.0) (`KismetMathLibrary.MakeRotator` 0.0 0.0 _returnvalue_yaw_2)) "None" false)))
      (:`SpawnAttack`
        (for _array_element_3 (`self.Meshes`)
          (bind (_returnvalue_roll_3 _returnvalue_pitch_3 _returnvalue_yaw_3) (`KismetMathLibrary.BreakRotator` (`KismetMathLibrary.FindLookAtRotation` (`self.K2_GetActorLocation`) (`SceneComponent.K2_GetComponentLocation` _array_element_3))))
          (bind _returnvalue_2 (`|SpawnActorFromClass` "/Game/Gameplay/Attacks/EnemyAttacks/BP_EnemySpawnerProjectile.BP_EnemySpawnerProjectile_C" (`KismetMathLibrary.MakeTransform` (+ (`SceneComponent.K2_GetComponentLocation` _array_element_3) (`KismetMathLibrary.GreaterGreater_VectorRotator` (10.0 0.0 0.0) (`KismetMathLibrary.MakeRotator` 0.0 0.0 _returnvalue_yaw_3)))) "Undefined" "OverrideRootScale" null null))
          (set `/Game/Gameplay/Attacks/EnemyAttacks/BP_EnemySpawnerProjectile.SpawnEnemy` true _returnvalue_2)
          (set `/Game/Gameplay/Attacks/BP_ProjectileParent.Shooter` self _returnvalue_2)
          (`PrimitiveComponent.AddImpulse` (`/Game/Gameplay/Attacks/BP_ProjectileParent.PhysicsCube` _returnvalue_2) (`KismetMathLibrary.GreaterGreater_VectorRotator` (1000.0 0.0 0.0) (`KismetMathLibrary.MakeRotator` 0.0 0.0 _returnvalue_yaw_3)) "None" false)))
      (:`LaserAttack`
        (if (== (`self.Shots`) 1)
          (`|ExecutionSequence`
            (:`then_0`
              (goto _label :!via `Stop`))
            (:`then_1`
              (bind (_direction_2 _yaw_2) (`Timeline|Laser` :!via `PlayFromStart`)
                (:`Update`
                  (`SceneComponent.K2_SetRelativeRotation` (`self.Rotator`) (`KismetMathLibrary.MakeRotator` 0.0 0.0 _yaw_2) false false)
                  (for _array_element_4 (`self.Meshes`)
                    (bind _outactors (`GameplayStatics.GetAllActorsOfClass` "/Game/NPCs/Enemies/BP_EnemyParent.BP_EnemyParent_C"))
                    (bind _returnvalue_3 (`SceneComponent.K2_GetComponentLocation` _array_element_4))
                    (bind (_returnvalue_roll_4 _returnvalue_pitch_4 _returnvalue_yaw_4) (`KismetMathLibrary.BreakRotator` (`SceneComponent.K2_GetComponentRotation` _array_element_4)))
                    (bind _outhits (`KismetSystemLibrary.LineTraceMulti` _returnvalue_3 (+ _returnvalue_3 (`KismetMathLibrary.GreaterGreater_VectorRotator` (1000.0 0.0 0.0) (`KismetMathLibrary.MakeRotator` 0.0 0.0 _returnvalue_yaw_4))) "TraceTypeQuery2" false _outactors "ForOneFrame" true (struct :`R` 1.0 :`A` 1.0) (struct :`G` 1.0 :`A` 1.0) 1.0))
                    (for _array_element_5 _outhits
                      (if (== (`.HitActor` (`GameplayStatics.BreakHitResult` _array_element_5)) (`GameplayStatics.GetPlayerCharacter` 0))
                        (`|ExecutionSequence`
                          (:`then_0`
                            (`KismetSystemLibrary.PrintString` "HALT YOUVE VIOLATED THE LAW"))
                          (:`then_1`
                            (break)))))))
                (:`Finished`
                  (set `self.Shots` 0)
                  (goto _label))))))))))

(event `self.ReceiveDestroyed`
  (for _index (range 5)
    (`|SpawnActorFromClass` "/Game/NPCs/Enemies/Test/BP_TestEnemy01.BP_TestEnemy01_C" (`KismetMathLibrary.MakeTransform` (+ (`self.K2_GetActorLocation`) (`KismetMathLibrary.GreaterGreater_VectorRotator` (300.0 0.0 0.0) (`KismetMathLibrary.MakeRotator` 0.0 0.0 (/ (* _index 360.0) 5.0))))) "Undefined" "OverrideRootScale" null null)))

(fn `UserConstructionScript`
  (`parent.UserConstructionScript`))