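; Base enemy Blueprint that handles trading hits with the player and dropping orbs when destroyed.
; Attack events set the Attacker on the victim's BPStatsComponent, then call Hit on the player or itself.
; BeginPlay grants a very brief invincibility window.
; On destruction, a nonzero stats State spawns several weapon orbs carrying that State, plus a health orb if DropState is set.
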(event `PerformAttack`
  ;[1 1 1] Attacking the player
  (bind _asbp_player (cast `/Game/Player/PlayerBlueprint/BP_Player` (`GameplayStatics.GetPlayerCharacter` 0)))
  (set `/Game/Gameplay/BP_StatsComponent.Attacker` self (`/Game/Gameplay/BP_CharacterParent.BP_StatsComponent` _asbp_player))
  (`self.Hit` _asbp_player))

(event `Player Has Attacked`
  ;[1 1 1] Getting Attacked By Player
  (bind _asbp_player (cast `/Game/Player/PlayerBlueprint/BP_Player` (`GameplayStatics.GetPlayerCharacter` 0)))
  (set `/Game/Gameplay/BP_StatsComponent.Attacker` _asbp_player (`self.BP_StatsComponent`))
  (`self.Hit`))

(event `self.ReceiveBeginPlay`
  (bind _bp_statscomponent (`self.BP_StatsComponent`))
  (set `/Game/Gameplay/BP_StatsComponent.Invincible` true _bp_statscomponent)
  (`KismetSystemLibrary.Delay` 0.01)
  (set `/Game/Gameplay/BP_StatsComponent.Invincible` false _bp_statscomponent))

(event `self.ReceiveDestroyed`
  (bind _bp_statscomponent (`self.BP_StatsComponent`))
  ;[1 1 1] Dropping
  (`|ExecutionSequence`
    (:`then_0`
      (if (and (`self.DropState`) (> (`/Game/Gameplay/BP_StatsComponent.State` _bp_statscomponent) 0))
        (`|SpawnActorFromClass` "/Game/Gameplay/Orbs/BP_HealthOrbParent.BP_HealthOrbParent_C" (`KismetMathLibrary.MakeTransform` (`self.K2_GetActorLocation`) (struct) (0.5 0.5 0.5)) "Undefined" "OverrideRootScale" null null)))
    (:`then_1`
      (if (not (== (`/Game/Gameplay/BP_StatsComponent.State` _bp_statscomponent) 0))
        (for _ (range 6)
          (bind _returnvalue (`|SpawnActorFromClass` "/Game/Gameplay/Orbs/BP_WeaponOrbParent.BP_WeaponOrbParent_C" (`KismetMathLibrary.MakeTransform` (`self.K2_GetActorLocation`) (struct) (0.2 0.2 0.2)) "Undefined" "OverrideRootScale" null null))
          (set `/Game/Gameplay/Orbs/BP_WeaponOrbParent.WeaponState` (`/Game/Gameplay/BP_StatsComponent.State` (`self.BP_StatsComponent`)) _returnvalue))))))

(fn `UserConstructionScript`
  (`parent.UserConstructionScript`))