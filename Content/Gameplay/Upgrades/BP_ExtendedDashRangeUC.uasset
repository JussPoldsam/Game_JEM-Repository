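; Upgrade Blueprint that extends the dash range of the player character.
; On activation it casts player 0's character to BP_Player and sets its DashLengthBonus along X, choosing the larger bonus when Power is zero and the smaller one otherwise.
; When the upgrade is destroyed, it resets that bonus to zero.
; The bonus is assigned outright, replacing any existing value.
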(event `self.UpgradeActivate`
  (bind _asbp_player (cast `/Game/Player/PlayerBlueprint/BP_Player` (`GameplayStatics.GetPlayerCharacter` 0)))
  (if (== (`self.Power`) 0)
    (set `/Game/Player/PlayerBlueprint/BP_Player.DashLengthBonus` (75.0 0.0 0.0) _asbp_player)
    (else
      (set `/Game/Player/PlayerBlueprint/BP_Player.DashLengthBonus` (50.0 0.0 0.0) _asbp_player))))

(event `self.UpgradeDestroyed`
  (bind _asbp_player (cast `/Game/Player/PlayerBlueprint/BP_Player` (`GameplayStatics.GetPlayerCharacter` 0)))
  (set `/Game/Player/PlayerBlueprint/BP_Player.DashLengthBonus` (0.0 0.0 0.0) _asbp_player))