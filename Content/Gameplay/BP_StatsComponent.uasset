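; Actor component that holds combat stats and resolves damage taken from an Attacker's own stats component.
; CalculateHealth skips invincible owners, then sums base, fire, arcane and dark damage after resistances, with toggles for elemental types, scaled by the attacker's multiplier.
; The player receives the result through PlayerHit unless dashing.
; Other owners lose Health directly and are destroyed at zero or below.
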(event `self.ReceiveBeginPlay`
  (set `self.MaxHealth` (`self.Health`)))

(event `CalculateHealth`
  (bind _returnvalue (`self.GetOwner`))
  (bind _returnvalue_2 (`Actor.GetComponentByClass` (`self.Attacker`) "BP_StatsComponent_C"))
  (bind _asbp_player (cast `/Game/Player/PlayerBlueprint/BP_Player` (`GameplayStatics.GetPlayerCharacter` 0) :!pure true))
  (bind _returnvalue_3 (* (+ (* (`/Game/Gameplay/BP_StatsComponent.BaseDmg` _returnvalue_2) (/ (- 100.0 (`self.BaseResistance`)) 100.0)) (* (`/Game/Gameplay/BP_StatsComponent.FireDmg` _returnvalue_2) (/ (- 100.0 (`self.FireResistance`)) 100.0) (`KismetMathLibrary.Conv_BoolToDouble` (`self.TakeFireDmg`))) (* (`/Game/Gameplay/BP_StatsComponent.ArcaneDmg` _returnvalue_2) (/ (- 100.0 (`self.ArcaneResistance`)) 100.0) (`KismetMathLibrary.Conv_BoolToDouble` (`self.TakeArcaneDmg`))) (* (`/Game/Gameplay/BP_StatsComponent.DarkDmg` _returnvalue_2) (/ (- 100.0 (`self.DarkResistance`)) 100.0) (`KismetMathLibrary.Conv_BoolToDouble` (`self.TakeDarkDmg`)))) (`/Game/Gameplay/BP_StatsComponent.AttackMultiplier` _returnvalue_2)))
  (if (`self.Invincible`)
    _
    (elif (== (`self.GetOwner`) _asbp_player)
      (if (not (`/Game/Player/PlayerBlueprint/BP_Player.Dashing` _asbp_player))
        (`/Game/Player/PlayerBlueprint/BP_Player.PlayerHit` _asbp_player _returnvalue_3))
      (else
        (bind _output_get (set `self.Health` (- (`self.Health`) _returnvalue_3)))
        (`KismetSystemLibrary.PrintString` (`KismetStringLibrary.Conv_DoubleToString` _output_get))
        (if (<= _output_get 0.0)
          (if (!= _returnvalue (`GameplayStatics.GetPlayerCharacter` 0))
            (`Actor.K2_DestroyActor` _returnvalue)))))))