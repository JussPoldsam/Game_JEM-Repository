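; Parent Blueprint for weapon orb pickups that fly to the player and award elemental weapon points.
; On spawn, the physics sphere gets a randomized upward and outward impulse, angled relative to the player-to-orb direction.
; After a short random delay, physics stops and a timeline lerps the orb onto the player's live location.
; On arrival, WeaponState selects whether BP_Player gains a clamped Fire, Arcane or Dark point, or none, then the orb destroys itself.
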(event `self.ReceiveBeginPlay`
  (bind (_returnvalue_roll _returnvalue_pitch _returnvalue_yaw) (`KismetMathLibrary.BreakRotator` (`KismetMathLibrary.FindLookAtRotation` (`self.K2_GetActorLocation` (`GameplayStatics.GetPlayerCharacter` 0)) (`self.K2_GetActorLocation`))))
  (bind (_returnvalue_x _returnvalue_y) (`KismetMathLibrary.BreakVector` (`KismetMathLibrary.GreaterGreater_VectorRotator` (`KismetMathLibrary.MakeVector` (+ (* (`KismetMathLibrary.RandomFloat`) 25.0) 25.0)) (`KismetMathLibrary.MakeRotator` _returnvalue_roll _returnvalue_pitch (+ (- _returnvalue_yaw 135.0) (* (`KismetMathLibrary.RandomFloat`) 225.0))))))
  (`PrimitiveComponent.AddImpulse` (`self.Sphere`) (`KismetMathLibrary.MakeVector` _returnvalue_x _returnvalue_y (+ (* (`KismetMathLibrary.RandomFloat`) 50.0) 25.0)) "None" false)
  (`KismetSystemLibrary.Delay` (`KismetMathLibrary.RandomFloatInRange` 0.4 0.6))
  (set `self.StartLocation` (`self.K2_GetActorLocation`))
  (`PrimitiveComponent.SetSimulatePhysics` (`self.Sphere`) false)
  (bind (_direction _newtrack_0) (`Timeline|TravelCurve`)
    (:`Update`
      (`self.K2_SetActorLocation` (`KismetMathLibrary.VLerp` (`self.StartLocation`) (`self.K2_GetActorLocation` (`GameplayStatics.GetPlayerCharacter` 0)) _newtrack_0)))
    (:`Finished`
      (bind _asbp_player (cast `/Game/Player/PlayerBlueprint/BP_Player` (`GameplayStatics.GetPlayerCharacter` 0)))
      (`|MultiGate` false false (`self.WeaponState`)
        (:`Out 0`
          (`self.K2_DestroyActor`))
        (:`Out 1`
          (set `/Game/Player/PlayerBlueprint/BP_Player.FirePoints` (`KismetMathLibrary.FClamp` (+ (`/Game/Player/PlayerBlueprint/BP_Player.FirePoints` _asbp_player) 1.0) 0.0 100.0) _asbp_player)
          (`self.K2_DestroyActor` :!label _label))
        (:`Out 2`
          (set `/Game/Player/PlayerBlueprint/BP_Player.ArcanePoints` (`KismetMathLibrary.FClamp` (+ (`/Game/Player/PlayerBlueprint/BP_Player.ArcanePoints` _asbp_player) 1.0) 0.0 100.0) _asbp_player)
          (goto _label))
        (:`Out 3`
          (set `/Game/Player/PlayerBlueprint/BP_Player.DarkPoints` (`KismetMathLibrary.FClamp` (+ (`/Game/Player/PlayerBlueprint/BP_Player.DarkPoints` _asbp_player) 1.0) 0.0 100.0) _asbp_player)
          (goto _label))))))

(fn `UserConstructionScript`)