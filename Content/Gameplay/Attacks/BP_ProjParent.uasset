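; Parent projectile for attacks fired by either the player or other shooters, with an optional timed self-destruct on spawn.
; A physics cube handles blocking hits that destroy it, while a box overlap resolves targets based on the Shooter.
; Player shots hit enemies or trigger health orbs; other shots hit the player unless invincible.
; For character hits, it registers itself as the stats component's Attacker before calling Hit, then destroys itself.
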(event `self.ReceiveBeginPlay`
  (if (`self.Decay`)
    (`KismetSystemLibrary.Delay` (`self.DecayTime`))
    (`self.K2_DestroyActor`)))

(event `self.PhysicsCube.OnComponentHit`
  (params (HitComponent :type "PrimitiveComponent Object Reference") (OtherActor :type "Actor Object Reference") (OtherComp :type "PrimitiveComponent Object Reference") (NormalImpulse :type "Vector Structure") (Hit :type "HitResult Structure (by ref)"))
  (if (not (== OtherActor null))
    (`self.K2_DestroyActor`)))

(event `self.BoxCollision.OnComponentBeginOverlap`
  (params (OverlappedComponent :type "PrimitiveComponent Object Reference") (OtherActor :type "Actor Object Reference") (OtherComp :type "PrimitiveComponent Object Reference") (OtherBodyIndex :type Integer) (bFromSweep :type Boolean) (SweepResult :type "HitResult Structure (by ref)"))
  (bind _returnvalue (`GameplayStatics.GetPlayerCharacter` 0))
  (if (== (`self.Shooter`) (`GameplayStatics.GetPlayerCharacter` 0))
    (bind _asbp_enemy_parent (cast `/Game/NPCs/Enemies/BP_EnemyParent` OtherActor)
      (:`then`
        (if (== _asbp_enemy_parent OtherActor)
          (bind _asbp_enemy_parent_2 (cast `/Game/NPCs/Enemies/BP_EnemyParent` OtherActor))
          (set `/Game/Gameplay/BP_StatsComponent.Attacker` self (`/Game/Gameplay/BP_CharacterParent.BP_StatsComponent` _asbp_enemy_parent_2))
          (`/Game/Gameplay/BP_CharacterParent.Hit` _asbp_enemy_parent_2)
          (`self.K2_DestroyActor`)
          (else
            (bind _asbp_health_orb_parent (cast `/Game/Gameplay/Orbs/BP_HealthOrbParent` OtherActor :!label _label))
            (if (== OtherActor _asbp_health_orb_parent)
              (`/Game/Gameplay/Orbs/BP_HealthOrbParent.PlayerHit` _asbp_health_orb_parent)
              (`self.K2_DestroyActor`)))))
      (:`CastFailed`
        (goto _label)))
    (elif (== OtherActor _returnvalue)
      (bind _asbp_player (cast `/Game/Player/PlayerBlueprint/BP_Player` _returnvalue))
      (bind _bp_statscomponent (`/Game/Gameplay/BP_CharacterParent.BP_StatsComponent` _asbp_player))
      (if (not (`/Game/Gameplay/BP_StatsComponent.Invincible` _bp_statscomponent))
        (set `/Game/Gameplay/BP_StatsComponent.Attacker` self _bp_statscomponent)
        (`/Game/Gameplay/BP_CharacterParent.Hit` _asbp_player)
        (`self.K2_DestroyActor`)))))

(fn `UserConstructionScript`)