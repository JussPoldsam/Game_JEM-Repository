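; Enemy attack actor that sweeps a beam outward from an origin to damage the player, with damage type and color set by its stats state.
; After an optional delay and guide lines, a timeline moves both beam endpoints along separate directions at separate speeds, destroying the actor once the source passes range.
; Instead of collision, which it removes, every other update uses yaw and distance math to hit a non-dashing, non-invincible player.
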(event `self.ReceiveBeginPlay`
  (bind _indicator1 (`self.Indicator1`))
  (bind _indicator2 (`self.Indicator2`))
  (bind _beamparticle (`self.BeamParticle`))
  (bind _bp_statscomponent (`self.BP_StatsComponent`))
  (bind _asmain_game_instance (cast `/Game/Player/PlayerBlueprint/MainGameInstance` (`GameplayStatics.GetGameInstance`) :!pure true))
  (bind _asmain_game_instance_2 (cast `/Game/Player/PlayerBlueprint/MainGameInstance` (`GameplayStatics.GetGameInstance`) :!pure true))
  (`parent.ReceiveBeginPlay`)
  (set `self.Player BP` (cast `/Game/Player/PlayerBlueprint/BP_Player` (`GameplayStatics.GetPlayerCharacter` 0) :!pure true))
  (`KismetSystemLibrary.Delay` 0.0)
  (switch `int` (`/Game/Gameplay/BP_StatsComponent.State` _bp_statscomponent)
    (:`0`
      _)
    (:`1`
      (set `/Game/Gameplay/BP_StatsComponent.FireDmg` 40.0 _bp_statscomponent)
      (set `/Game/Gameplay/BP_StatsComponent.BaseDmg` 0.0 _bp_statscomponent :!label _label))
    (:`2`
      (set `/Game/Gameplay/BP_StatsComponent.ArcaneDmg` 40.0 _bp_statscomponent)
      (goto _label))
    (:`3`
      (set `/Game/Gameplay/BP_StatsComponent.DarkDmg` 40.0 _bp_statscomponent)
      (goto _label)))
  ;[1 1 1] Set Particle Color
  (switch `int` (`/Game/Gameplay/BP_StatsComponent.State` (`self.BP_StatsComponent`))
    (:`0`
      _)
    (:`1`
      (`ParticleSystemComponent.SetColorParameter` _beamparticle "CustomColor" (`/Game/Player/PlayerBlueprint/MainGameInstance.FireColor` _asmain_game_instance))
      (for _array_element (`|MakeArray` (`self.Indicator1`) (`self.Indicator2`)) :!label _label_2
        (switch `int` (`/Game/Gameplay/BP_StatsComponent.State` (`self.BP_StatsComponent`))
          (:`1`
            (`ParticleSystemComponent.SetColorParameter` _array_element "CustomColor" (`/Game/Player/PlayerBlueprint/MainGameInstance.FireColor` _asmain_game_instance_2)))
          (:`2`
            (`ParticleSystemComponent.SetColorParameter` _array_element "CustomColor" (`/Game/Player/PlayerBlueprint/MainGameInstance.ArcaneColor` _asmain_game_instance_2)))
          (:`3`
            (`ParticleSystemComponent.SetColorParameter` _array_element "CustomColor" (`/Game/Player/PlayerBlueprint/MainGameInstance.DarkColor` _asmain_game_instance_2))))))
    (:`2`
      (`ParticleSystemComponent.SetColorParameter` _beamparticle "CustomColor" (`/Game/Player/PlayerBlueprint/MainGameInstance.ArcaneColor` _asmain_game_instance))
      (goto _label_2))
    (:`3`
      (`ParticleSystemComponent.SetColorParameter` _beamparticle "CustomColor" (`/Game/Player/PlayerBlueprint/MainGameInstance.DarkColor` _asmain_game_instance))
      (goto _label_2)))
  (if (`self.DrawLines`)
    (`SceneComponent.SetVisibility` (`self.Indicator1`) true false)
    (`SceneComponent.SetVisibility` (`self.Indicator2`) true false)
    (`ParticleSystemComponent.SetBeamSourcePoint` _indicator1 0 (+ (`self.OriginLocation`) (`KismetMathLibrary.GreaterGreater_VectorRotator` (`KismetMathLibrary.MakeVector` (`self.AttackStartDistance`)) (`KismetMathLibrary.MakeRotator` 0.0 0.0 (`self.SourceDirection`)))) 0)
    (`ParticleSystemComponent.SetBeamTargetPoint` _indicator1 0 (+ (`self.OriginLocation`) (`KismetMathLibrary.GreaterGreater_VectorRotator` (2000.0 0.0 0.0) (`KismetMathLibrary.MakeRotator` 0.0 0.0 (`self.SourceDirection`)))) 0)
    (`ParticleSystemComponent.SetBeamSourcePoint` _indicator2 0 (+ (`self.OriginLocation`) (`KismetMathLibrary.GreaterGreater_VectorRotator` (`KismetMathLibrary.MakeVector` (`self.AttackStartDistance`)) (`KismetMathLibrary.MakeRotator` 0.0 0.0 (`self.TargetDirection`)))) 0)
    (`ParticleSystemComponent.SetBeamTargetPoint` _indicator2 0 (+ (`self.OriginLocation`) (`KismetMathLibrary.GreaterGreater_VectorRotator` (2000.0 0.0 0.0) (`KismetMathLibrary.MakeRotator` 0.0 0.0 (`self.TargetDirection`)))) 0))
  (if (> (`self.StartDelay`) 0.0)
    (`|ExecutionSequence`
      (:`then_0`
        (`ParticleSystemComponent.SetBeamSourcePoint` (`self.BeamParticle`) 0 (+ (`self.OriginLocation`) (`KismetMathLibrary.GreaterGreater_VectorRotator` (`KismetMathLibrary.MakeVector` (`self.AttackStartDistance`)) (`KismetMathLibrary.MakeRotator` 0.0 0.0 (`self.SourceDirection`)))) 0)
        (`ParticleSystemComponent.SetBeamTargetPoint` (`self.BeamParticle`) 0 (+ (`self.OriginLocation`) (`KismetMathLibrary.GreaterGreater_VectorRotator` (`KismetMathLibrary.MakeVector` (`self.AttackStartDistance`)) (`KismetMathLibrary.MakeRotator` 0.0 0.0 (`self.TargetDirection`)))) 0))
      (:`then_1`
        (`KismetSystemLibrary.Delay` (`self.StartDelay`))
        (`self.Attack` :!label _label_3)))
    (else
      (goto _label_3))))

(event `Attack`
  (bind _player_bp (`self.Player BP`))
  (bind (_sourcepoint_x _sourcepoint_y) (`KismetMathLibrary.BreakVector` (`self.SourcePoint`)))
  (bind (_targetpoint_x _targetpoint_y) (`KismetMathLibrary.BreakVector` (`self.TargetPoint`)))
  (bind _sourcepoint (`self.SourcePoint`))
  (bind _targetpoint (`self.TargetPoint`))
  (bind _player_bp_2 (`self.Player BP`))
  (bind (_returnvalue_x _returnvalue_y) (`KismetMathLibrary.BreakVector` (`self.K2_GetActorLocation` (`GameplayStatics.GetPlayerCharacter` 0))))
  (bind (_returnvalue_roll _returnvalue_pitch _returnvalue_yaw) (`KismetMathLibrary.BreakRotator` (`KismetMathLibrary.FindLookAtRotation` _targetpoint (`self.SourcePoint`))))
  (bind (_returnvalue_roll_2 _returnvalue_pitch_2 _returnvalue_yaw_2) (`KismetMathLibrary.BreakRotator` (`KismetMathLibrary.FindLookAtRotation` _sourcepoint (`self.TargetPoint`))))
  (bind _returnvalue (- _returnvalue_x _sourcepoint_x))
  (bind _returnvalue_2 (- _returnvalue_y _sourcepoint_y))
  (bind (_returnvalue_roll_3 _returnvalue_pitch_3 _returnvalue_yaw_3) (`KismetMathLibrary.BreakRotator` (`KismetMathLibrary.FindLookAtRotation` _targetpoint (`self.K2_GetActorLocation` (`GameplayStatics.GetPlayerCharacter` 0)))))
  (bind _returnvalue_3 (`KismetMathLibrary.ClampAxis` _returnvalue_yaw))
  (bind (_returnvalue_roll_4 _returnvalue_pitch_4 _returnvalue_yaw_4) (`KismetMathLibrary.BreakRotator` (`KismetMathLibrary.FindLookAtRotation` _sourcepoint (`self.K2_GetActorLocation` (`GameplayStatics.GetPlayerCharacter` 0)))))
  (bind _returnvalue_4 (`KismetMathLibrary.ClampAxis` _returnvalue_yaw_2))
  (bind _returnvalue_5 (`KismetMathLibrary.ClampAxis` _returnvalue_yaw_3))
  (bind _returnvalue_6 (`KismetMathLibrary.ClampAxis` _returnvalue_yaw_4))
  (`|ExecutionSequence`
    (:`then_0`
      (bind (_direction _alpha) (`Timeline|SetLocation` :!via `PlayFromStart`)
        (:`Update`
          (bind _returnvalue_7 (`KismetMathLibrary.Lerp` (`self.AttackStartDistance`) (`self.AttackEndDistance`) (* _alpha (`self.SourceSpeed`))))
          (if (> _returnvalue_7 3000.0)
            (`self.K2_DestroyActor`)
            (else
              (set `self.SourcePoint` (+ (`self.OriginLocation`) (`KismetMathLibrary.GreaterGreater_VectorRotator` (`KismetMathLibrary.MakeVector` _returnvalue_7) (`KismetMathLibrary.MakeRotator` 0.0 0.0 (`self.SourceDirection`)))))
              (`ParticleSystemComponent.SetBeamSourcePoint` (`self.BeamParticle`) 0 (`self.SourcePoint`) 0)
              (set `self.TargetPoint` (+ (`self.OriginLocation`) (`KismetMathLibrary.GreaterGreater_VectorRotator` (`KismetMathLibrary.MakeVector` (`KismetMathLibrary.Lerp` (`self.AttackStartDistance`) (`self.AttackEndDistance`) (* _alpha (`self.TargetSpeed`)))) (`KismetMathLibrary.MakeRotator` 0.0 0.0 (`self.TargetDirection`)))))
              (`ParticleSystemComponent.SetBeamTargetPoint` (`self.BeamParticle`) 0 (`self.TargetPoint`) 0)
              (`/Engine/EditorBlueprintResources/StandardMacros.FlipFlop`
                (:`A`
                  (if (or (`/Game/Gameplay/BP_StatsComponent.Invincible` (`/Game/Gameplay/BP_CharacterParent.BP_StatsComponent` _player_bp)) (`/Game/Player/PlayerBlueprint/BP_Player.Dashing` _player_bp))
                    _
                    (elif (< _returnvalue_6 (+ _returnvalue_4 90.0))
                      (if (> _returnvalue_6 (- _returnvalue_4 90.0))
                        (if (< _returnvalue_5 (+ _returnvalue_3 90.0))
                          (if (> _returnvalue_5 (- _returnvalue_3 90.0))
                            (if (< (* (/ (`KismetMathLibrary.VSize` (`KismetMathLibrary.MakeVector` _returnvalue _returnvalue_2)) 2.0) (`KismetMathLibrary.DegSin` (`KismetMathLibrary.DegAcos` (`KismetMathLibrary.Dot_VectorVector` (`KismetMathLibrary.Normal` (`KismetMathLibrary.MakeVector` _returnvalue _returnvalue_2)) (`KismetMathLibrary.Normal` (`KismetMathLibrary.MakeVector` (- _targetpoint_x _sourcepoint_x) (- _targetpoint_y _sourcepoint_y))))))) 20.0)
                              (set `/Game/Gameplay/BP_StatsComponent.Attacker` self (`/Game/Gameplay/BP_CharacterParent.BP_StatsComponent` _player_bp_2))
                              (`/Game/Gameplay/BP_CharacterParent.Hit` _player_bp_2))))))))))))))
    (:`then_1`
      (if (`self.DrawLines`)
        (`KismetSystemLibrary.Delay` 2.3)
        (`ActorComponent.K2_DestroyComponent` (`self.Indicator1`))
        (`ActorComponent.K2_DestroyComponent` (`self.Indicator2`))))))

(fn `UserConstructionScript`
  (`parent.UserConstructionScript`)
  (`ActorComponent.K2_DestroyComponent` (`self.BoxCollision`))
  (`ActorComponent.K2_DestroyComponent` (`self.PhysicsCube`)))