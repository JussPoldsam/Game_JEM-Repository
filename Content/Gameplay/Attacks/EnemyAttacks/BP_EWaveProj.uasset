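; Enemy wave attack projectile that sends a particle beam outward from its spawn location.
; After a start delay, a timeline lerps distance from start to end, scaled by attack speed.
; Each update rotates that distance by source and target yaws to place the beam's endpoints, so the beam spans two diverging directions.
; The construction script destroys the BoxCollision and PhysicsCube components, and this graph contains no hit or damage logic.
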(event `self.ReceiveBeginPlay`
  (`parent.ReceiveBeginPlay`)
  ;[1 0.03292 0] MUST BE SET WHEN CREATED
  (set `self.OriginLocation` (`self.K2_GetActorLocation`))
  (`KismetSystemLibrary.Delay` (`self.StartDelay`))
  (`self.Attack`))

(event `Attack`
  (bind (_direction _alpha) (`Timeline|SetLocation` :!via `PlayFromStart`)
    (:`Update`
      (bind _returnvalue (* _alpha (`self.AttackSpeed`)))
      (set `self.SourcePoint` (+ (`self.OriginLocation`) (`KismetMathLibrary.GreaterGreater_VectorRotator` (`KismetMathLibrary.MakeVector` (`KismetMathLibrary.Lerp` (`self.AttackStartDistance`) (`self.AttackEndDistance`) _returnvalue)) (`KismetMathLibrary.MakeRotator` 0.0 0.0 (`self.SourceDirection`)))))
      (`ParticleSystemComponent.SetBeamSourcePoint` (`self.ParticleSystem`) 0 (`self.SourcePoint`) 0)
      (set `self.TargetPoint` (+ (`self.OriginLocation`) (`KismetMathLibrary.GreaterGreater_VectorRotator` (`KismetMathLibrary.MakeVector` (`KismetMathLibrary.Lerp` (`self.AttackStartDistance`) (`self.AttackEndDistance`) _returnvalue)) (`KismetMathLibrary.MakeRotator` 0.0 0.0 (`self.TargetDirection`)))))
      (`ParticleSystemComponent.SetBeamTargetPoint` (`self.ParticleSystem`) 0 (`self.TargetPoint`) 0))))

(fn `UserConstructionScript`
  (`parent.UserConstructionScript`)
  (`ActorComponent.K2_DestroyComponent` (`self.BoxCollision`))
  (`ActorComponent.K2_DestroyComponent` (`self.PhysicsCube`)))