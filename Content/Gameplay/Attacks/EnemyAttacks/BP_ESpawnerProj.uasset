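; BP_ESpawnerProj is an enemy attack projectile with a physics cube that can turn into an enemy.
; After BeginPlay, if SpawnEnemy is set and fewer than 50 BP_TestEnemy01 exist, it waits four seconds, spawns one at the cube's location and destroys itself.
; At the cap it does neither.
; With SpawnEnemy off, it only sets linear damping on the cube.
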(event `self.ReceiveBeginPlay`
  (`parent.ReceiveBeginPlay`)
  (`KismetSystemLibrary.Delay` 0.01)
  (if (`self.SpawnEnemy`)
    (bind _outactors (`GameplayStatics.GetAllActorsOfClass` "/Game/NPCs/Enemies/Test/BP_TestEnemy01.BP_TestEnemy01_C"))
    (if (< (`KismetArrayLibrary.Array_Length` _outactors) 50)
      (`KismetSystemLibrary.Delay` 4.0)
      (`|SpawnActorFromClass` "/Game/NPCs/Enemies/Test/BP_TestEnemy01.BP_TestEnemy01_C" (`KismetMathLibrary.MakeTransform` (`SceneComponent.K2_GetComponentLocation` (`self.PhysicsCube`))) "AlwaysSpawn" "OverrideRootScale" null null)
      (`self.K2_DestroyActor`))
    (else
      (`PrimitiveComponent.SetLinearDamping` (`self.PhysicsCube`) 0.45))))

(fn `UserConstructionScript`
  (`parent.UserConstructionScript`))