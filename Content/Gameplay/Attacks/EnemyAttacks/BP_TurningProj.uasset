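; Enemy attack projectile that glides out to a wall or maximum range, then becomes a turning laser aimed at the player.
; MoveTo timeline drives the glide, then a state-colored indicator beam appears.
; Tracking timeline swings the beam from backward toward the player's current position, updating traces on alternate ticks.
; Fire locks the final direction, swaps in the laser, and only upon hitting world geometry damages the player and self-destructs.
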(event `self.ReceiveBeginPlay`
  (bind _returnvalue (`self.K2_GetActorLocation`))
  (bind _indicatorbeam (`self.IndicatorBeam`))
  (bind _indicatorbeam_2 (`self.IndicatorBeam`))
  (bind _asmain_game_instance (cast `/Game/Player/PlayerBlueprint/MainGameInstance` (`GameplayStatics.GetGameInstance`) :!pure true))
  (`parent.ReceiveBeginPlay`)
  (`KismetSystemLibrary.Delay` 0.0)
  ;[1 1 1] Set Particle Color
  (switch `int` (`/Game/Gameplay/BP_StatsComponent.State` (`self.BP_StatsComponent`))
    (:`0`
      _)
    (:`1`
      (`ParticleSystemComponent.SetColorParameter` _indicatorbeam "CustomColor" (`/Game/Player/PlayerBlueprint/MainGameInstance.FireColor` _asmain_game_instance)))
    (:`2`
      (`ParticleSystemComponent.SetColorParameter` _indicatorbeam "CustomColor" (`/Game/Player/PlayerBlueprint/MainGameInstance.ArcaneColor` _asmain_game_instance)))
    (:`3`
      (`ParticleSystemComponent.SetColorParameter` _indicatorbeam "CustomColor" (`/Game/Player/PlayerBlueprint/MainGameInstance.DarkColor` _asmain_game_instance))))
  (set `self.StartingLocation` _returnvalue)
  (bind (_outhit _returnvalue_2) (`KismetSystemLibrary.LineTraceSingleForObjects` _returnvalue (+ _returnvalue (`KismetMathLibrary.GreaterGreater_VectorRotator` (1000.0 0.0 0.0) (`KismetMathLibrary.MakeRotator` 0.0 0.0 (`self.StartDirection`)))) (`|MakeArray` "ObjectTypeQuery1" :!type "EObjectTypeQuery Enum")))
  (if _returnvalue_2
    (set `self.MoveToLocation` (`.Location` (`GameplayStatics.BreakHitResult` _outhit)))
    (bind (_direction _alpha) (`Timeline|MoveTo` :!via `PlayFromStart` :!label _label)
      (:`Update`
        (`self.K2_SetActorLocation` (`KismetMathLibrary.VLerp` (`self.StartingLocation`) (`self.MoveToLocation`) _alpha)))
      (:`Finished`
        (`SceneComponent.SetVisibility` _indicatorbeam_2 true false)
        (`ParticleSystemComponent.SetBeamSourcePoint` _indicatorbeam_2 0 (`self.K2_GetActorLocation`) 0)
        (`ParticleSystemComponent.SetBeamTargetPoint` _indicatorbeam_2 0 (`self.StartingLocation`) 0)
        (`KismetSystemLibrary.Delay` 0.7)
        (`self.Track`)))
    (else
      (set `self.MoveToLocation` (`.TraceEnd` (`GameplayStatics.BreakHitResult` _outhit)))
      (goto _label :!via `PlayFromStart`))))

(event `Track`
  (bind _returnvalue (`self.K2_GetActorLocation`))
  (bind _indicatorbeam (`self.IndicatorBeam`))
  (bind (_returnvalue_roll _returnvalue_pitch _returnvalue_yaw) (`KismetMathLibrary.BreakRotator` (`KismetMathLibrary.FindLookAtRotation` (`self.K2_GetActorLocation`) (`self.K2_GetActorLocation` (`GameplayStatics.GetPlayerCharacter` 0)))))
  (bind (_direction _alpha) (`Timeline|Tracking` :!via `PlayFromStart`)
    (:`Update`
      (`/Engine/EditorBlueprintResources/StandardMacros.FlipFlop`
        (:`A`
          (bind (_returnvalue_roll_2 _returnvalue_pitch_2 _returnvalue_yaw_2) (`KismetMathLibrary.BreakRotator` (`KismetMathLibrary.RLerp` (`KismetMathLibrary.MakeRotator` 0.0 0.0 (+ (`self.StartDirection`) 180.0)) (`KismetMathLibrary.MakeRotator` 0.0 0.0 _returnvalue_yaw) _alpha true)))
          (bind (_outhit _returnvalue_2) (`KismetSystemLibrary.LineTraceSingleForObjects` _returnvalue (+ _returnvalue (`KismetMathLibrary.GreaterGreater_VectorRotator` (4000.0 0.0 0.0) (`KismetMathLibrary.MakeRotator` 0.0 0.0 _returnvalue_yaw_2))) (`|MakeArray` "ObjectTypeQuery1" :!type "EObjectTypeQuery Enum")))
          (if _returnvalue_2
            (`ParticleSystemComponent.SetBeamTargetPoint` _indicatorbeam 0 (`.Location` (`GameplayStatics.BreakHitResult` _outhit)) 0)
            (else
              (`ParticleSystemComponent.SetBeamTargetPoint` _indicatorbeam 0 (`.TraceEnd` (`GameplayStatics.BreakHitResult` _outhit)) 0))))))
    (:`Finished`
      (set `self.TrackEndLocation` (`ParticleSystemComponent.GetBeamTargetPoint` (`self.IndicatorBeam`) 0 0))
      (`KismetSystemLibrary.Delay` 0.2)
      (`self.Fire`))))

(event `Fire`
  (bind _returnvalue (`self.K2_GetActorLocation`))
  (bind _returnvalue_2 (`GameplayStatics.GetPlayerCharacter` 0))
  (bind _indicatorbeam (`self.IndicatorBeam`))
  (bind (_returnvalue_roll _returnvalue_pitch _returnvalue_yaw) (`KismetMathLibrary.BreakRotator` (`KismetMathLibrary.FindLookAtRotation` (`self.K2_GetActorLocation`) (`self.TrackEndLocation`))))
  (bind _asbp_player (cast `/Game/Player/PlayerBlueprint/BP_Player` _returnvalue_2 :!pure true))
  (`ParticleSystemComponent.SetTemplate` (`self.IndicatorBeam`) "/Game/Particles/Test/P_ELaser.P_ELaser")
  (bind (_outhit _returnvalue_3) (`KismetSystemLibrary.LineTraceSingleForObjects` _returnvalue (+ _returnvalue (`KismetMathLibrary.GreaterGreater_VectorRotator` (5000.0 0.0 0.0) (`KismetMathLibrary.MakeRotator` 0.0 0.0 _returnvalue_yaw))) (`|MakeArray` "ObjectTypeQuery1" :!type "EObjectTypeQuery Enum")))
  (if _returnvalue_3
    (`ParticleSystemComponent.SetBeamTargetPoint` _indicatorbeam 0 (`.Location` (`GameplayStatics.BreakHitResult` _outhit)) 0)
    (bind _outhits (`KismetSystemLibrary.LineTraceMultiForObjects` (`self.K2_GetActorLocation`) (`ParticleSystemComponent.GetBeamTargetPoint` (`self.IndicatorBeam`) 0 0) (`|MakeArray` "ObjectTypeQuery3" :!type "EObjectTypeQuery Enum")))
    (for _array_element _outhits
      (if (== (`.HitActor` (`GameplayStatics.BreakHitResult` _array_element)) _returnvalue_2)
        (`|ExecutionSequence`
          (:`then_0`
            (set `/Game/Gameplay/BP_StatsComponent.Attacker` self (`/Game/Gameplay/BP_CharacterParent.BP_StatsComponent` _asbp_player))
            (`/Game/Gameplay/BP_CharacterParent.Hit` _asbp_player))
          (:`then_1`
            (break)))))
    (`KismetSystemLibrary.Delay` 0.3)
    (`self.K2_DestroyActor`)
    (else
      (`ParticleSystemComponent.SetBeamTargetPoint` _indicatorbeam 0 (`.TraceEnd` (`GameplayStatics.BreakHitResult` _outhit)) 0))))

(fn `UserConstructionScript`
  (`parent.UserConstructionScript`)
  (`ActorComponent.K2_DestroyComponent` (`self.BoxCollision`))
  (`ActorComponent.K2_DestroyComponent` (`self.PhysicsCube`)))