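; Enemy homing projectile that slowly tracks the player, then commits to a fast straight charge.
; A timeline moves PhysicsCube without sweep, steering MomentumYaw toward the player by a sine of the angle difference, scaled by the absolute look-at yaw.
; After a short delay, once roughly aligned, it locks its heading onto the player's predicted position, using velocity and distance, and stops homing.
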(event `self.ReceiveBeginPlay`
  (bind _returnvalue (`GameplayStatics.GetPlayerCharacter` 0))
  (bind _physicscube (`self.PhysicsCube`))
  (bind _physicscube_2 (`self.PhysicsCube`))
  (bind _returnvalue_2 (`SceneComponent.K2_GetComponentLocation` (`self.PhysicsCube`)))
  (bind _returnvalue_3 (`self.K2_GetActorLocation` _returnvalue))
  (bind (_returnvalue_roll _returnvalue_pitch _returnvalue_yaw) (`KismetMathLibrary.BreakRotator` (`KismetMathLibrary.FindLookAtRotation` (`SceneComponent.K2_GetComponentLocation` (`self.PhysicsCube`)) (`self.K2_GetActorLocation` (`GameplayStatics.GetPlayerCharacter` 0)))))
  (bind (_returnvalue_roll_2 _returnvalue_pitch_2 _returnvalue_yaw_2) (`KismetMathLibrary.BreakRotator` (`KismetMathLibrary.FindLookAtRotation` (`SceneComponent.K2_GetComponentLocation` (`self.PhysicsCube`)) (`self.K2_GetActorLocation` (`GameplayStatics.GetPlayerCharacter` 0)))))
  (bind (_returnvalue_roll_3 _returnvalue_pitch_3 _returnvalue_yaw_3) (`KismetMathLibrary.BreakRotator` (`KismetMathLibrary.FindLookAtRotation` _returnvalue_2 (+ _returnvalue_3 (* (`self.GetVelocity` _returnvalue) (/ (`KismetMathLibrary.VSize` (- _returnvalue_2 _returnvalue_3)) 400.0))))))
  (`parent.ReceiveBeginPlay`)
  (`|ExecutionSequence`
    (:`then_0`
      (`Timeline|SetLocation`
        (:`Update`
          (if (`self.Charging`)
            (`SceneComponent.K2_SetWorldLocation` _physicscube_2 (+ (`SceneComponent.K2_GetComponentLocation` _physicscube_2) (`KismetMathLibrary.GreaterGreater_VectorRotator` (15.0 0.0 0.0) (`KismetMathLibrary.MakeRotator` 0.0 0.0 (`self.MomentumYaw`)))) false false)
            (else
              (set `self.MomentumYaw` (+ (`self.MomentumYaw`) (* (/ (`KismetMathLibrary.ClampAxis` _returnvalue_yaw_2) 100.0) (`KismetMathLibrary.DegSin` (- _returnvalue_yaw_2 (`self.MomentumYaw`))))))
              (`SceneComponent.K2_SetWorldLocation` _physicscube (+ (`SceneComponent.K2_GetComponentLocation` _physicscube) (`KismetMathLibrary.GreaterGreater_VectorRotator` (4.0 0.0 0.0) (`KismetMathLibrary.MakeRotator` 0.0 0.0 (`self.MomentumYaw`)))) false false)
              (if (`self.CanCharge`)
                (if (<= (`KismetMathLibrary.Abs` (- (`KismetMathLibrary.ClampAxis` (`self.MomentumYaw`)) (`KismetMathLibrary.ClampAxis` _returnvalue_yaw))) 10.0)
                  (set `self.Charging` true)
                  (set `self.MomentumYaw` _returnvalue_yaw_3))))))))
    (:`then_1`
      (`KismetSystemLibrary.Delay` 2.0)
      (set `self.CanCharge` true))))

(fn `UserConstructionScript`
  (`parent.UserConstructionScript`))