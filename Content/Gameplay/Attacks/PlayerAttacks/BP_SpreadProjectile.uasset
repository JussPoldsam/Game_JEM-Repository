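; BP_SpreadProjectile is a player attack projectile that bursts into a cone of eight weaker copies of itself shortly after spawning.
; On BeginPlay, the first generation takes the player's attack yaw and splits after a short delay.
; Split spawns children at its physics cube with a fraction of its damage, launches them by impulse across a narrow arc, then destroys itself.
; A generation counter stops the children from splitting again.
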(event `self.ReceiveBeginPlay`
  (if (== (`self.Generation`) 0)
    (bind _asbp_player (cast `/Game/Player/PlayerBlueprint/BP_Player` (`GameplayStatics.GetPlayerCharacter` 0)))
    (set `self.AttackDirection` (`/Game/Player/PlayerBlueprint/BP_Player.AttackYawDirection` _asbp_player))
    (`self.DetermineSplit`))
  (`parent.ReceiveBeginPlay`))

(event `DetermineSplit`
  (`KismetSystemLibrary.Delay` 0.01)
  (if (== (`self.Generation`) 0)
    (`KismetSystemLibrary.Delay` 0.2)
    (`self.Split`)))

(event `Split`
  (for _index (range 8)
    (bind _returnvalue (`|SpawnActorFromClass` "BP_SpreadProjectile_C" (`KismetMathLibrary.MakeTransform` (`SceneComponent.K2_GetComponentLocation` (`self.PhysicsCube`))) "AlwaysSpawn" "OverrideRootScale" null null))
    (set `/Game/Gameplay/Attacks/BP_ProjectileParent.Shooter` (`self.Shooter`) _returnvalue)
    (set `/Game/Gameplay/BP_CharacterParent.BaseDamage` (* (`self.BaseDamage`) 0.2) _returnvalue)
    (set `/Game/Gameplay/Attacks/PlayerAttacks/BP_SpreadProjectile.Generation` (+ (`self.Generation`) 1) _returnvalue)
    (set `/Game/Gameplay/Attacks/PlayerAttacks/BP_SpreadProjectile.AttackDirection` 0.0 _returnvalue)
    (`PrimitiveComponent.AddImpulse` (`/Game/Gameplay/Attacks/BP_ProjectileParent.PhysicsCube` _returnvalue) (`KismetMathLibrary.GreaterGreater_VectorRotator` (2400.0 0.0 0.0) (`KismetMathLibrary.MakeRotator` 0.0 0.0 (+ (`self.AttackDirection`) -15.0 (/ (* _index 30.0) 8.0)))) "None" false))
  (`self.K2_DestroyActor`))

(fn `UserConstructionScript`
  (`parent.UserConstructionScript`))